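; Flying spectator Blueprint for free-camera movement along the camera's forward, right and up axes, with optional VR support.
; Mouse look yaws the controller and pitches a spring arm, but is ignored with an HMD, which V toggles.
; BeginPlay sets rotation lag and pawn control rotation according to HMD state.
; Inputs scale a clamped speed applied as player character MaxAcceleration, while custom events step the clamped field of view.
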(event `Event_Increase_FOV`
  (bind _firstpersoncamera (`self.FirstPersonCamera`))
  ;[1 1 1] Adjust Field of View
  (set `CameraComponent.FieldOfView` (`KismetMathLibrary.FClamp` (+ (`CameraComponent.FieldOfView` _firstpersoncamera) 5.0) 45.0 120.0) _firstpersoncamera))

(event `Key|V`
  (params (Key :type "Key Structure" :default "AnyKey"))
  (:`Pressed`
    (`/Engine/EditorBlueprintResources/StandardMacros.FlipFlop`
      (:`A`
        (`HeadMountedDisplayFunctionLibrary.EnableHMD` false))
      (:`B`
        (`HeadMountedDisplayFunctionLibrary.EnableHMD` true)))))

(event `Event_Decrease_FOV`
  (bind _firstpersoncamera (`self.FirstPersonCamera`))
  ;[1 1 1] Adjust Field of View
  (set `CameraComponent.FieldOfView` (`KismetMathLibrary.FClamp` (- (`CameraComponent.FieldOfView` _firstpersoncamera) 5.0) 45.0 120.0) _firstpersoncamera))

(event `self.ReceiveBeginPlay`
  (if (`HeadMountedDisplayFunctionLibrary.IsHeadMountedDisplayEnabled`)
    (set `SpringArmComponent.CameraRotationLagSpeed` 0.0 (`self.SpringArm`))
    (set `CameraComponent.bUsePawnControlRotation` true (`self.FirstPersonCamera`))
    (else
      (set `SpringArmComponent.CameraRotationLagSpeed` 5.0 (`self.SpringArm`))
      (set `CameraComponent.bUsePawnControlRotation` false (`self.FirstPersonCamera`)))))

(event `InputAxis|Turn`
  (params (AxisValue :type "Float (single-precision)"))
  ;[1 1 1] Rotation
  (if (not (`HeadMountedDisplayFunctionLibrary.IsHeadMountedDisplayEnabled`))
    (`self.AddControllerYawInput` (* (* AxisValue (`self.MouseSpeed`)) 0.65))))

(event `InputAction|Increase_Speed`
  (params (Key :type "Key Structure" :default "AnyKey"))
  ;[1 1 1] Change Speed
  (:`Pressed`
    (bind _output_get (set `self.Speed` (`KismetMathLibrary.FClamp` (* (`self.Speed`) 1.4) (`self.MinSpeed`) (`self.MaxSpeed`))))
    (set `CharacterMovementComponent.MaxAcceleration` _output_get (`Character.CharacterMovement` (`GameplayStatics.GetPlayerCharacter` 0)))))

(event `InputAxis|MoveForward`
  (params (AxisValue :type "Float (single-precision)"))
  ;[1 1 1] Movement
  (`self.AddMovementInput` (`SceneComponent.GetForwardVector` (`PlayerCameraManager.TransformComponent` (`GameplayStatics.GetPlayerCameraManager` 0))) AxisValue))

(event `InputAxis|MoveRight`
  (params (AxisValue :type "Float (single-precision)"))
  ;[1 1 1] Movement
  (`self.AddMovementInput` (`SceneComponent.GetRightVector` (`PlayerCameraManager.TransformComponent` (`GameplayStatics.GetPlayerCameraManager` 0))) AxisValue))

(event `InputAxis|LookUp`
  (params (AxisValue :type "Float (single-precision)"))
  ;[1 1 1] Rotation
  (if (not (`HeadMountedDisplayFunctionLibrary.IsHeadMountedDisplayEnabled`))
    (`SceneComponent.K2_AddRelativeRotation` (`self.SpringArm`) (`KismetMathLibrary.MakeRotator` 0.0 (* (* AxisValue (`self.MouseSpeed`)) -1.0)) false false)))

(event `InputAction|Decrease_Speed`
  (params (Key :type "Key Structure" :default "AnyKey"))
  ;[1 1 1] Change Speed
  (:`Pressed`
    (bind _output_get (set `self.Speed` (`KismetMathLibrary.FClamp` (/ (`self.Speed`) 1.4) (`self.MinSpeed`) (`self.MaxSpeed`))))
    (set `CharacterMovementComponent.MaxAcceleration` _output_get (`Character.CharacterMovement` (`GameplayStatics.GetPlayerCharacter` 0)))))

(event `InputAxis|MoveUp`
  (params (AxisValue :type "Float (single-precision)"))
  ;[1 1 1] Movement
  (`self.AddMovementInput` (`SceneComponent.GetUpVector` (`PlayerCameraManager.TransformComponent` (`GameplayStatics.GetPlayerCameraManager` 0))) AxisValue))

(fn `UserConstructionScript`
  (set `CameraComponent.FieldOfView` (`self.Field of View`) (`self.FirstPersonCamera`)))