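; Spawner that populates a radius around itself with BP_CrabMonster AI pawns on BeginPlay, unless spawning is disabled.
; A delayed event loop picks random navigable points, retries failures, and passes tuning properties to each crab, optionally dividing roar chance by the remaining count.
; Spawned crabs get default controllers and are tracked in an array for bulk destruction.
; The construction script saves the initial count so StartSpawn can repeat the batch.
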(event `Event_StartSpawn`
  (bind _amount_to_spawn (`self.Amount_to_Spawn`))
  (bind _chance_of_roar (`self.Chance_of_Roar`))
  (bind _returnvalue (`NavigationSystem.GetRandomPointInNavigableRadius` (`self.K2_GetActorLocation`) (`self.Spawn Radius`)))
  ;[1 1 1] Reset the amount to Spawn and then start spawning
  (set `self.Amount_to_Spawn` (`self.Amount_to_Spawn_Reset`))
  (if (not (`self.DisableSpawning?`)) :!label _label
    ;[1 1 1] Spawn Pawn in random Navigable point. Then add it to the Array
    (if (`AIBlueprintHelperLibrary.IsValidAILocation` _returnvalue) :!label _label_2
      (bind _returnvalue_2 (`|SpawnActorFromClass` "/Game/CrabMonster/Blueprints/BP_CrabMonster.BP_CrabMonster_C" (`KismetMathLibrary.MakeTransform` (`KismetMathLibrary.MakeVector` (.x _returnvalue) (.y _returnvalue) (+ (.z _returnvalue) 200.0)) (`KismetMathLibrary.MakeRotator` 0.0 0.0 (`KismetMathLibrary.RandomFloatInRange` 0.0 360.0))) "Undefined" "OverrideRootScale" null (`self.Speed`) (`self.Glow_Color`) (`self.Glowing_PointLight`) (`self.Glow_Light_Intensity`) (`self.Roaming_Radius`) (`self.A.I_HearingRadius_Absoloute`) (`self.A.I_HearingRadius_Unoccluded`) (`self.A.I_SightRadius`) (`KismetMathLibrary.SelectFloat` (/ _chance_of_roar (`KismetMathLibrary.Conv_IntToDouble` (`self.Amount_to_Spawn`))) _chance_of_roar (`self.ChanceOfRoar_BasedOn_SpawnAmount`)) (`self.Chance_of_Idle_Tapping`) (`self.Scale_Minimum`) (`self.Scale_Maximum`) (`self.Scale_Affects_Sensing_Distance`) (`self.Glow_Light_Radius`) (`self.A.I_Speed_Variation`) (`self.Glowing_Eye`) (`self.Maximum_Roaming_Angle`) (`self.Aggressiveness_Level`) (`self.A.I_Growl_Warning_Time`) (`self.Chance_of_Roar_WhileGrowling_At_Player`) (`self.Run_WhileChasing`)))
      (`/Engine/EditorBlueprintResources/StandardMacros.IsValid` _returnvalue_2
        (:`Is Valid`
          (`Pawn.SpawnDefaultController` _returnvalue_2)
          (`KismetArrayLibrary.Array_Add` (`self.Spawned_Pawns`) _returnvalue_2)
          ;[1 1 1] Subtract 1 from the amount of Pawns to Spawn (unless the amount is 1), and then Spawn again
          (if (!= _amount_to_spawn 1)
            (set `self.Amount_to_Spawn` (- _amount_to_spawn 1))
            (`KismetSystemLibrary.Delay` (`self.Spawn_Delay`) :!label _label_3)
            (`self.Event_SpawnAnother`)))
        (:`Is Not Valid`
          (goto _label_3)))
      (else
        (`KismetSystemLibrary.Delay` 0.1) ; If not a valid location, pick another random point
        (goto _label_2)))))

(event `self.ReceiveBeginPlay`
  (goto _label))

(event `Event_SpawnAnother`
  (goto _label))

(event `Event_DestroySpawnedActors`
  (bind _spawned_pawns (`self.Spawned_Pawns`))
  ;[1 0 0] Destroy All Spawned Actors
  (for _array_element _spawned_pawns
    (`/Engine/EditorBlueprintResources/StandardMacros.IsValid` _array_element
      (:`Is Valid`
        (`self.K2_DestroyActor` _array_element))))
  (`KismetArrayLibrary.Array_Clear` _spawned_pawns))

(fn `UserConstructionScript`
  (set `self.Amount_to_Spawn_Reset` (`self.Amount_to_Spawn`)) ; We store the amount to Spawn at the beginning, so we can use it to respawn that same amount later
)