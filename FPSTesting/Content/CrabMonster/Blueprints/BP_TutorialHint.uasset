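; BP_TutorialHint is a world-placed tutorial hint that swaps between a spinning icon and multi-line text by player proximity.
; Construction joins TextLines into the text render and sizes the backdrop.
; Tick turns the hint toward the camera and uses paired DoOnce gates on pawn distance to play or reverse one scaling timeline.
; Tick also shrinks the backdrop to near zero every frame, despite the timeline scaling it.
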(event `self.ReceiveBeginPlay`)

(event `self.ReceiveActorBeginOverlap`
  (params (OtherActor :type "Actor Object Reference")))

(event `self.ReceiveTick`
  (params (DeltaSeconds :type "Float (single-precision)"))
  (`SceneComponent.K2_AddWorldRotation` (`self.Icon`) (struct :`Yaw` 2.0) false false) ; Spin the icon
  (`self.Make Text look at player`)
  (`self.Toggle Visibily of Text and Hint Icon`)
  (`SceneComponent.SetWorldScale3D` (`self.Backdrop`) (0.001 0.001 0.001)) ; Hide Backdrop
)

(event `Event_OpenHint`
  (bind (_direction _text_scale _icon_scale) (`Timeline|Timeline_OpenHint` :!label _label)
    (:`Update`
      (`SceneComponent.SetWorldScale3D` (`self.TextRender`) (`KismetMathLibrary.Conv_DoubleToVector` _text_scale))
      (`SceneComponent.SetWorldScale3D` (`self.Icon`) (`KismetMathLibrary.Conv_DoubleToVector` _icon_scale))
      (`SceneComponent.SetWorldScale3D` (`self.Backdrop`) (`KismetMathLibrary.VLerp` (0.001 0.001 0.001) (`self.Backdrop_Scale`) _text_scale)))))

(event `Event_CloseHint`
  (goto _label :!via `Reverse`))

(fn `Make Text look at player`
  (`SceneComponent.K2_SetWorldRotation` (`self.Backdrop`) (`KismetMathLibrary.FindLookAtRotation` (`SceneComponent.K2_GetComponentLocation` (`self.TextRender`)) (`PlayerCameraManager.GetCameraLocation` (`GameplayStatics.GetPlayerCameraManager` 0))) false false)
  (`SceneComponent.K2_SetWorldRotation` (`self.Rotation`) (`KismetMathLibrary.FindLookAtRotation` (`SceneComponent.K2_GetComponentLocation` (`self.TextRender`)) (`PlayerCameraManager.GetCameraLocation` (`GameplayStatics.GetPlayerCameraManager` 0))) false false))

(fn `Toggle Visibily of Text and Hint Icon`
  (if (< (`KismetMathLibrary.VSize` (- (`self.K2_GetActorLocation` (`GameplayStatics.GetPlayerPawn` 0)) (`SceneComponent.K2_GetComponentLocation` (`self.TextRender`)))) (`self.Distance_to_Show_Text`))
    (`/Engine/EditorBlueprintResources/StandardMacros.DoOnce` false :!label _label
      (:`Completed`
        (`self.Event_OpenHint`)
        (goto _label_2 :!via `Reset`)))
    (else
      (`/Engine/EditorBlueprintResources/StandardMacros.DoOnce` false :!label _label_2
        (:`Completed`
          (`self.Event_CloseHint`)
          (goto _label :!via `Reset`))))))

(fn `UserConstructionScript`
  (bind _textlines (`self.TextLines`))
  (bind _returnvalue (`KismetMathLibrary.MakeVector` 1.0 (`self.Backdrop_X`) (`self.Backdrop_Y`)))
  (`SceneComponent.SetWorldScale3D` (`self.Backdrop`) _returnvalue)
  (set `self.Backdrop_Scale` _returnvalue)
  (for (_array_element _array_index) _textlines
    (if (!= _array_index (`KismetArrayLibrary.Array_LastIndex` _textlines))
      (set `self.Text` (`KismetStringLibrary.Concat_StrStr` (`self.Text`) (`KismetStringLibrary.Concat_StrStr` _array_element " \n")))
      (else
        (set `self.Text` (`KismetStringLibrary.Concat_StrStr` (`self.Text`) _array_element)))))
  (`TextRenderComponent.K2_SetText` (`self.TextRender`) (`KismetTextLibrary.Conv_StringToText` (`self.Text`))))